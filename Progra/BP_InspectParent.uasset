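; Base Blueprint for an inspectable object, letting an inspector rotate its Item component with the mouse.
; StartInspect moves player input from the Inspector to this actor.
; While either left or right mouse button is held, mouse X and Y add scaled, inverted roll and pitch to Item's relative rotation via CombineRotators.
; Pressing Interact returns input to the Inspector and calls Inspect on it as a ThirdPersonCharacter.
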(event Custom|StartInspect
  (params (Inspector :type Pawn%20Object%20Reference))
  (bind _returnvalue (Game|GetPlayerController 0))
  ;[1 1 1] StartRotator
  (Input|DisableInput Inspector _returnvalue)
  (Input|EnableInput _returnvalue))

(event EventBeginPlay)

(event Input|ActionEvents|InputActionInteract
  (params (Key :type Key%20Structure :default "None"))
  (bind _returnvalue (Game|GetPlayerController 0))
  ;[1 1 1] StartRotator
  (:Pressed
    (Input|DisableInput _returnvalue)
    (Input|EnableInput (stale Custom|StartInspect Inspector) _returnvalue)
    (bind _asthird_person_character (Utilities|Casting|CastToThirdPersonCharacter (stale Custom|StartInspect Inspector)))
    (Default|Inspect _asthird_person_character)))

(event Input|MouseEvents|MouseX
  (params (AxisValue :type Float%20%28single-precision%29))
  (bind _returnvalue (Game|GetPlayerController 0))
  (if (or (Game|Player|IsInputKeyDown _returnvalue "LeftMouseButton") (Game|Player|IsInputKeyDown _returnvalue "RightMouseButton"))
    (Transformation|SetRelativeRotation (Variables|Default|GetItem) (Math|Rotator|CombineRotators (Variables|/Script/Engine.SceneComponent|GetRelativeRotation (Variables|Default|GetItem)) (Math|Rotator|MakeRotator (* AxisValue -1.5) 0.0 0.0)) false false)))

(event Input|MouseEvents|MouseY
  (params (AxisValue :type Float%20%28single-precision%29))
  (bind _returnvalue (Game|GetPlayerController 0))
  (if (or (Game|Player|IsInputKeyDown _returnvalue "LeftMouseButton") (Game|Player|IsInputKeyDown _returnvalue "RightMouseButton"))
    (Transformation|SetRelativeRotation (Variables|Default|GetItem) (Math|Rotator|CombineRotators (Variables|/Script/Engine.SceneComponent|GetRelativeRotation (Variables|Default|GetItem)) (Math|Rotator|MakeRotator 0.0 (* AxisValue -1.5) 0.0)) false false)))

(fn ConstructionScript)