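; Interactable locker with a three-digit code lock that ends the game when opened.
; Overlapping InteractArea with MC_BP shows a widget; interacting while locked opens Code_Widget with the digits and a self reference, switching to UI input.
; CheckCode compares the concatenated digits to Codigo, opening on a match or playing a tap sound otherwise.
; Opening plays sound and confetti, shows EndGame_Widget, then quits after a delay.
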(event OnComponentBeginOverlap(InteractArea)
  (params (OverlappedComponent :type Primitive%20Component%20Object%20Reference) (OtherActor :type Actor%20Object%20Reference) (OtherComp :type Primitive%20Component%20Object%20Reference) (OtherBodyIndex :type Integer) (bFromSweep :type Boolean) (SweepResult :type Hit%20Result%20Structure%20%28by%20ref%29))
  (Utilities|Casting|CastToMC_BP OtherActor)
  (Rendering|SetVisibility (Variables|Default|GetWidget) true false))

(event OnComponentEndOverlap(InteractArea)
  (params (OverlappedComponent :type Primitive%20Component%20Object%20Reference) (OtherActor :type Actor%20Object%20Reference) (OtherComp :type Primitive%20Component%20Object%20Reference) (OtherBodyIndex :type Integer))
  (Utilities|Casting|CastToMC_BP OtherActor)
  (Rendering|SetVisibility (Variables|Default|GetWidget) false false))

(event Custom|OpenSafe
  (Variables|CodeAtt|SetIsLocked false)
  (Variables|CodeAtt|SetIsOpen true)
  (Audio|SpawnSound2D "/Game/Progra/Locker/SFXLocker/LockerOpen.LockerOpen" 1.0 1.0 0.0 0)
  (Effects|SpawnEmitteratLocation "/Game/Progra/Locker/Confetti/ConfettiEmitter.ConfettiEmitter" (Transformation|GetWorldLocation (Variables|Default|GetSpawner)))
  (bind _returnvalue (UserInterface|CreateWidget "/Game/Progra/Locker/EndGame_Widget.EndGame_Widget_C"))
  (UserInterface|Viewport|AddtoViewport _returnvalue 0)
  (Utilities|FlowControl|Delay 5.0)
  (Game|QuitGame 0 "Quit" false))

(event EventInteract
  (bind _returnvalue (Game|GetPlayerController 0))
  (if (not (Variables|CodeAtt|GetIsOpen))
    (if (Variables|CodeAtt|GetIsLocked)
      (bind _returnvalue_2 (UserInterface|CreateWidget "/Game/Progra/Locker/Code_Widget.Code_Widget_C" 0 (Variables|GenerateCode|GetDigit1) (Variables|GenerateCode|GetDigit2) (Variables|GenerateCode|GetDigit3) self))
      (bind _output_get (Variables|Default|SetCodeUI _returnvalue_2))
      (UserInterface|Viewport|AddtoViewport _output_get 3)
      (Input|SetInputModeUIOnly _returnvalue _output_get "DoNotLock")
      (Variables|/Script/Engine.PlayerController|SetbShowMouseCursor _returnvalue true)
      (else
        (CallFunction|OpenSafe)))))

(fn ConstructionScript)

(fn CheckCode
  (bind _returnvalue (Game|GetPlayerController 0))
  (Variables|GenerateCode|SetGenerateCode "")
  (Variables|GenerateCode|SetGenerateCode (Utilities|String|Append (Utilities|String|ToString(Integer) (Variables|GenerateCode|GetDigit1)) (Utilities|String|ToString(Integer) (Variables|GenerateCode|GetDigit2)) (Utilities|String|ToString(Integer) (Variables|GenerateCode|GetDigit3))))
  (if (Utilities|Enum|Equal(Enum) (Variables|CodeAtt|GetCodigo) (Variables|GenerateCode|GetGenerateCode))
    (Development|PrintString "OPEN")
    (CallFunction|OpenSafe)
    (Widget|RemovefromParent (Variables|Default|GetCodeUI))
    (Variables|Default|SetCodeUI 0)
    (Input|SetInputModeGameOnly _returnvalue)
    (Variables|/Script/Engine.PlayerController|SetbShowMouseCursor _returnvalue false)
    (else
      (Audio|SpawnSound2D "/Game/Progra/Locker/SFXLocker/LockerTapNumbers.LockerTapNumbers" 1.0 1.0 0.0 0))))